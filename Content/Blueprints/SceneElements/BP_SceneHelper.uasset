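; BP_SceneHelper is a scene setup helper that configures waypoints and agent spawners through two custom events.
; GenerateWayPointsIDs numbers every A_WayPoint by array index and shows the ID on its text renderer.
; FillAgentSpawnerData splits the total agent count evenly across all A_AgentSpawner actors and copies the shared spawn delay to each.
; It also adds every waypoint ID to each spawner's goal map with uniform probability, so it relies on those IDs.
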(event Custom|Generate%20WayPoints%20IDs
  (bind _outactors (Actor|GetAllActorsOfClass "/Game/Blueprints/SceneElements/A_WayPoint.A_WayPoint_C"))
  (for (_array_element _array_index) _outactors
    (bind _output_get (Variables|/Game/Blueprints/SceneElements/A_WayPoint.A_WayPoint_C|SetId _array_element _array_index))
    (Rendering|Components|TextRender|SetText (Variables|/Game/Blueprints/SceneElements/A_WayPoint.A_WayPoint_C|GetIdRenderer _array_element) (Utilities|Text|ToText(Integer) _output_get))))

(event Custom|Fill%20Agent%20Spawner%20Data
  (bind _outactors (Actor|GetAllActorsOfClass "/Game/Blueprints/SceneElements/A_AgentSpawner.A_AgentSpawner_C"))
  (for _array_element _outactors
    (Variables|/Game/Blueprints/SceneElements/A_AgentSpawner.A_AgentSpawner_C|SetAgents%20To%20Spawn _array_element (/ (Variables|Default|GetTotalAgentNumToSpawn) (Utilities|Array|Length _outactors)))
    (Variables|/Game/Blueprints/SceneElements/A_AgentSpawner.A_AgentSpawner_C|SetSpawnDelay _array_element (Variables|Default|GetSpawnDelay))
    (bind _outactors_2 (Actor|GetAllActorsOfClass "/Game/Blueprints/SceneElements/A_WayPoint.A_WayPoint_C"))
    (for _array_element_2 _outactors_2
      (Utilities|Map|Add (Variables|/Game/Blueprints/SceneElements/A_AgentSpawner.A_AgentSpawner_C|GetProbabilitiesOfGoals _array_element) (Variables|/Game/Blueprints/SceneElements/A_WayPoint.A_WayPoint_C|GetId _array_element_2) (/ 1.0 (Math|Conversions|ToFloat(Integer) (Utilities|Array|Length _outactors_2)))))))

(event EventBeginPlay)

(event Collision|EventActorBeginOverlap
  (params (OtherActor :type Actor%20Object%20Reference)))

(event EventTick
  (params (DeltaSeconds :type Float%20%28single-precision%29)))

(fn ConstructionScript)