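; BP_Camera is a player-controlled camera rig that pans, rotates and zooms through input axes.
; Forward and Right move the actor along its rotated local axes, while Rotate Right changes only its yaw.
; ZoomOut slides the Camera component along its relative offset, rejecting steps that bring it too close to the actor origin.
; The square root of that offset's length scales panning up and rotation down as the camera zooms out.
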(event EventBeginPlay)

(event Collision|EventActorBeginOverlap
  (params (OtherActor :type Actor%20Object%20Reference)))

(event EventTick
  (params (DeltaSeconds :type Float%20%28single-precision%29)))

(event Input|AxisEvents|InputAxisForward
  (params (AxisValue :type Float%20%28single-precision%29))
  (Transformation|SetActorLocation (+ (* (Math|Vector|RotateVector (* (Math|Vector|MakeVector (/ (Math|Float|Sqrt (Math|Vector|VectorLength (Variables|/Script/Engine.SceneComponent|GetRelativeLocation (Variables|Default|GetCamera)))) 5e+01) 0.0 0.0) AxisValue) (Transformation|GetActorRotation)) (Variables|Default|GetLinearSpeed)) (Transformation|GetActorLocation)) false false))

(event Input|AxisEvents|InputAxisRight
  (params (AxisValue :type Float%20%28single-precision%29))
  (Transformation|SetActorLocation (+ (* (Math|Vector|RotateVector (* (Math|Vector|MakeVector 0.0 (/ (Math|Float|Sqrt (Math|Vector|VectorLength (Variables|/Script/Engine.SceneComponent|GetRelativeLocation (Variables|Default|GetCamera)))) 5e+01) 0.0) AxisValue) (Transformation|GetActorRotation)) (Variables|Default|GetLinearSpeed)) (Transformation|GetActorLocation)) false false))

(event Input|AxisEvents|InputAxisRotateRight
  (params (AxisValue :type Float%20%28single-precision%29))
  (Transformation|SetActorRotation (Math|Rotator|MakeRotator 0.0 0.0 (+ (.Yaw (Math|Rotator|BreakRotator (* (* (Math|Rotator|MakeRotator 0.0 0.0 -1.0) (/ (Variables|Default|GetAngleSpeed) (Math|Float|Sqrt (Math|Vector|VectorLength (Variables|/Script/Engine.SceneComponent|GetRelativeLocation (Variables|Default|GetCamera)))))) AxisValue))) (.Yaw (Math|Rotator|BreakRotator (Transformation|GetActorRotation)))))))

(event Input|AxisEvents|InputAxisZoomOut
  (params (AxisValue :type Float%20%28single-precision%29))
  (bind _camera (Variables|Default|GetCamera))
  (bind _zoomspeed (Variables|Default|GetZoomSpeed))
  (bind _relativelocation (Variables|/Script/Engine.SceneComponent|GetRelativeLocation _camera))
  (bind _relativelocation_2 (Variables|/Script/Engine.SceneComponent|GetRelativeLocation _camera))
  (bind _returnvalue (Math|Vector|Normalize _relativelocation_2))
  (bind _returnvalue_2 (* _returnvalue AxisValue))
  (bind _returnvalue_3 (* _returnvalue_2 _zoomspeed))
  (bind _returnvalue_4 (+ _returnvalue_3 _relativelocation))
  (if (> (Math|Vector|VectorLength _returnvalue_4) 3e+01)
    (Transformation|SetRelativeLocation (Variables|Default|GetCamera) _returnvalue_4 false false)))

(fn ConstructionScript)