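; Scene utility actor that rescales the level layout by a ResizeCoef factor when its Resize event is called.
; Static mesh actors get scaled X/Y locations with Z forced to zero, and scaled size with an extra ZScale multiplier on height.
; NavMeshBoundsVolume and Floor_Blueprint actors are then stretched in X and Y only, keeping their location and height scale.
; Each pass multiplies current transforms, so repeated calls compound.
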(event Custom|Resize
  (bind _resize_coef (Variables|Default|GetResize%20Coef))
  (bind _resize_coef_2 (Variables|Default|GetResize%20Coef))
  (bind _resize_coef_3 (Variables|Default|GetResize%20Coef))
  (Utilities|FlowControl|Sequence
    (:then_0
      (bind _outactors (Actor|GetAllActorsOfClass "/Script/Engine.StaticMeshActor"))
      (for _array_element _outactors
        (Transformation|SetActorTransform _array_element (Math|Transform|MakeTransform (Math|Vector|MakeVector (.X (Math|Vector|BreakVector (* (.Location (Math|Transform|BreakTransform (Transformation|GetActorTransform _array_element))) _resize_coef))) (.Y (Math|Vector|BreakVector (* (.Location (Math|Transform|BreakTransform (Transformation|GetActorTransform _array_element))) _resize_coef))) 0.0) (.Rotation (Math|Transform|BreakTransform (Transformation|GetActorTransform _array_element))) (Math|Vector|MakeVector (.X (Math|Vector|BreakVector (* (.Scale (Math|Transform|BreakTransform (Transformation|GetActorTransform _array_element))) _resize_coef))) (.Y (Math|Vector|BreakVector (* (.Scale (Math|Transform|BreakTransform (Transformation|GetActorTransform _array_element))) _resize_coef))) (* (.Z (Math|Vector|BreakVector (* (.Scale (Math|Transform|BreakTransform (Transformation|GetActorTransform _array_element))) _resize_coef))) (Variables|Default|GetZ%20Scale)))))))
    (:then_1
      (bind _outactors_2 (Actor|GetAllActorsOfClass "/Script/NavigationSystem.NavMeshBoundsVolume"))
      (for _array_element_2 _outactors_2
        (Transformation|SetActorTransform _array_element_2 (Math|Transform|MakeTransform (.Location (Math|Transform|BreakTransform (Transformation|GetActorTransform _array_element_2))) (.Rotation (Math|Transform|BreakTransform (Transformation|GetActorTransform _array_element_2))) (Math|Vector|MakeVector (* _resize_coef_3 (.X (Math|Vector|BreakVector (.Scale (Math|Transform|BreakTransform (Transformation|GetActorTransform _array_element_2)))))) (* _resize_coef_3 (.Y (Math|Vector|BreakVector (.Scale (Math|Transform|BreakTransform (Transformation|GetActorTransform _array_element_2)))))) (.Z (Math|Vector|BreakVector (.Scale (Math|Transform|BreakTransform (Transformation|GetActorTransform _array_element_2))))))))))
    (:then_2
      (bind _outactors_3 (Actor|GetAllActorsOfClass "/Game/Floor_Blueprint.Floor_Blueprint_C"))
      (for _array_element_3 _outactors_3
        (Transformation|SetActorTransform _array_element_3 (Math|Transform|MakeTransform (.Location (Math|Transform|BreakTransform (Transformation|GetActorTransform _array_element_3))) (.Rotation (Math|Transform|BreakTransform (Transformation|GetActorTransform _array_element_3))) (Math|Vector|MakeVector (* _resize_coef_2 (.X (Math|Vector|BreakVector (.Scale (Math|Transform|BreakTransform (Transformation|GetActorTransform _array_element_3)))))) (* _resize_coef_2 (.Y (Math|Vector|BreakVector (.Scale (Math|Transform|BreakTransform (Transformation|GetActorTransform _array_element_3)))))) (.Z (Math|Vector|BreakVector (.Scale (Math|Transform|BreakTransform (Transformation|GetActorTransform _array_element_3))))))))))))

(event EventBeginPlay)

(event Collision|EventActorBeginOverlap
  (params (OtherActor :type Actor%20Object%20Reference)))

(event EventTick
  (params (DeltaSeconds :type Float%20%28single-precision%29)))

(fn ConstructionScript)